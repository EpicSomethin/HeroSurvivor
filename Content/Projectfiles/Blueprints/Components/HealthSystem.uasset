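; HealthSystem component that sets up stats and starting health for its owning actor.
; InitStats copies each BaseStats data table row into the CurrentStats map, then seeds CurrentHealth from the MaxHealth entry.
; It also binds a handler to the owner's OnTakeAnyDamage.
; Damage handling is a stub: CustomTakeDamage and the auto-generated function are empty, and an ApplyDamage call is left unconnected.
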(event Custom|InitStats
  (bind _basestats (Variables|Default|GetBaseStats))
  (bind _outrownames (DataTable|GetDataTableRowNames _basestats))
  (for _array_element _outrownames
    (bind _returnvalue (Utilities|GetDataTableRow _basestats _array_element)
      (:then
        (Utilities|Map|Add (Variables|Default|GetCurrentStats) _array_element (.Value (Utilities|Struct|BreakStats _returnvalue))))))
  (Variables|Default|SetCurrentHealth (.Value (Utilities|Map|Find (Variables|Default|GetCurrentStats) "MaxHealth")))
  (EventDispatchers|BindEventtoOnTakeAnyDamage (Components|GetOwner) (EventDispatchers|CreateEvent :!event Custom|CustomTakeDamage)))

(event Custom|CustomTakeDamage
  (params (DamagedActor :type Actor%20Object%20Reference) (Damage :type Float%20%28single-precision%29) (DamageType :type Damage%20Type%20Object%20Reference) (InstigatedBy :type Controller%20Object%20Reference) (DamageCauser :type Actor%20Object%20Reference)))

(event EventBeginPlay)

(event EventTick
  (params (DeltaSeconds :type Float%20%28single-precision%29)))

(fn HealthSystemAutoGenFunc
  (params (DamagedActor :type Actor%20Object%20Reference) (Damage :type Float%20%28single-precision%29) (DamageType :type Damage%20Type%20Object%20Reference) (InstigatedBy :type Controller%20Object%20Reference) (DamageCauser :type Actor%20Object%20Reference)))