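; Actor component that manages its owner's stats and health, including typed damage and timed debuffs.
; InitStats loads base stats from a data table, and TickStats rebuilds final stats by layering flat then percent changes while preserving current health.
; ApplyDamage computes flat or health-based amounts, then mitigates physical and magical damage with armour and magic resist.
; A one-second timer ticks debuffs, and owner messages delegate effects and UI updates.
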(event Custom|InitStats
  (bind _basestatstable (Variables|Default|GetBaseStatsTable))
  (bind _basestats (Variables|Default|GetBaseStats))
  ;[1 1 1] Initialise Stats
  (bind _outrownames (DataTable|GetDataTableRowNames _basestatstable))
  (for _array_element _outrownames
    (bind _returnvalue (Utilities|GetDataTableRow _basestatstable _array_element)
      (:then
        (Utilities|Map|Add _basestats _array_element (.Value (Utilities|Struct|BreakStats _returnvalue))))))
  (Utilities|Map|Add (Variables|Default|GetFinalStats) "CurrentHealth" (.Value (Utilities|Map|Find _basestats "MaxHealth")))
  (Utilities|FlowControl|Delay 0.2)
  (CallFunction|TickStats)
  (Utilities|Time|SetTimerbyFunctionName 0 "TickStats" 1.0 true))

(event Custom|Update%20Stats%20UI
  (params (Stat%20To%20Update :type StatsEnum%20Enum :default "NewEnumerator0") (Update%20All? :type Boolean) (NumberToUpdate :type Float%20%28double-precision%29) (TextToUpdate :type String))
  ;[1 1 1] Allow Owner to determine Logic
  (Class|DamageSystem|OwnerUpdateUI(Message) (Components|GetOwner) Stat%20To%20Update Update%20All? NumberToUpdate TextToUpdate (Variables|Default|GetFinalStats)))

(event Custom|DamageEffects
  (params (FXType :type DamageFXTypeEnum%20Enum :default "NewEnumerator0") (DamageNumbers :type Float%20%28double-precision%29) (DamageNumerType :type DamageTypeEnum%20Enum :default "NewEnumerator0") (Color :type Slate%20Color%20Structure))
  ;[1 1 1] Allow Owner to determine Logic
  (Class|DamageSystem|DamageEffect(Message) (Components|GetOwner) FXType DamageNumbers DamageNumerType Color))

(event Custom|TickDebuffs
  (bind _debuff (Variables|Default|GetDebuff))
  (bind _debufflength (Variables|Default|GetDebuffLength))
  ;[0.4589 0.1573 1] DebuffLogic
  (bind _keys (Utilities|Map|Keys _debuff))
  (for _array_element _keys
    (Variables|Default|SetDebuffName _array_element)
    (Utilities|FlowControl|Sequence
      (:then_0
        (if (Utilities|Map|Contains _debufflength (Variables|Default|GetDebuffName))
          _
          (else
            (Utilities|Map|Add _debufflength (Variables|Default|GetDebuffName) (.LengthOfEntireDebuff (Utilities|Struct|BreakDebuff (.Value (Utilities|Map|Find _debuff (Variables|Default|GetDebuffName))))))))
        (if (== (.Value (Utilities|Map|Find _debufflength (Variables|Default|GetDebuffName))) 0.0)
          (switch Utilities|FlowControl|Switch|SwitchonDebuffEnum (.DebuffType (Utilities|Struct|BreakDebuff (.Value (Utilities|Map|Find _debuff (Variables|Default|GetDebuffName)))))
            (:NewEnumerator0
              _)
            (:NewEnumerator1
              (Utilities|Map|Remove (Variables|Default|GetFlatStatChanges) (Variables|Default|GetDebuffName))
              (CallFunction|TickStats))
            (:NewEnumerator2
              (Utilities|Map|Remove (Variables|Default|GetPercentStatChanges) (Variables|Default|GetDebuffName))
              (CallFunction|TickStats)))
          (Utilities|Map|Remove (Variables|Default|GetDebuff) (Variables|Default|GetDebuffName))
          (Utilities|Map|Remove (Variables|Default|GetDebuffLength) (Variables|Default|GetDebuffName))
          (else
            (bind _result (Math|Float|DecrementFloat (.Value (Utilities|Map|Find _debufflength (Variables|Default|GetDebuffName))))
              (:%20%20
                (Utilities|Map|Add _debufflength (Variables|Default|GetDebuffName) _result)
                (switch Utilities|FlowControl|Switch|SwitchonDebuffEnum (.DebuffType (Utilities|Struct|BreakDebuff (.Value (Utilities|Map|Find _debuff (Variables|Default|GetDebuffName)))))
                  (:NewEnumerator0
                    (CallFunction|ApplyDamage (.DamageAmount (Utilities|Struct|BreakDebuff (.Value (Utilities|Map|Find _debuff (Variables|Default|GetDebuffName))))) (.DamageAmount (Utilities|Struct|BreakDebuff (.Value (Utilities|Map|Find _debuff (Variables|Default|GetDebuffName))))) (.DamageAmount (Utilities|Struct|BreakDebuff (.Value (Utilities|Map|Find _debuff (Variables|Default|GetDebuffName))))) (.DamageType (Utilities|Struct|BreakDebuff (.Value (Utilities|Map|Find _debuff (Variables|Default|GetDebuffName))))) 0 0 (.DamageMethod (Utilities|Struct|BreakDebuff (.Value (Utilities|Map|Find _debuff (Variables|Default|GetDebuffName))))) (.DamagePercentage (Utilities|Struct|BreakDebuff (.Value (Utilities|Map|Find _debuff (Variables|Default|GetDebuffName))))))
                    (CallFunction|DamageEffects "NewEnumerator3" (.DamageAmount (Utilities|Struct|BreakDebuff (.Value (Utilities|Map|Find _debuff (Variables|Default|GetDebuffName))))) (.DamageType (Utilities|Struct|BreakDebuff (.Value (Utilities|Map|Find _debuff (Variables|Default|GetDebuffName)))))))
                  (:NewEnumerator1
                    (Utilities|Map|Add (Variables|Default|GetFlatStatChanges) (Variables|Default|GetDebuffName) (Utilities|Struct|MakeStatChangesFlat (.FlatReductionAmount (Utilities|Struct|BreakDebuff (.Value (Utilities|Map|Find _debuff (Variables|Default|GetDebuffName))))) (.StatToReduce (Utilities|Struct|BreakDebuff (.Value (Utilities|Map|Find _debuff (Variables|Default|GetDebuffName))))) (Variables|Default|GetDebuffName) false)))
                  (:NewEnumerator2
                    (Utilities|Map|Add (Variables|Default|GetPercentStatChanges) (Variables|Default|GetDebuffName) (Utilities|Struct|MakeStatChangesPercent (.PercentageReductionAmount (Utilities|Struct|BreakDebuff (.Value (Utilities|Map|Find _debuff (Variables|Default|GetDebuffName))))) (.StatToReduce (Utilities|Struct|BreakDebuff (.Value (Utilities|Map|Find _debuff (Variables|Default|GetDebuffName))))) (Variables|Default|GetDebuffName) false)))))))))
      (:then_1
        (CallFunction|TickStats)))))

(event Custom|ApplyPercentStatChanges
  (params (StatsToChange :type Map%20of%20Names%20to%20Reals) (CurrentPercentChanges :type Map%20of%20Names%20to%20Structs))
  ;[1 0.9092 0.4678] Update Stats Logic
  (bind _keys (Utilities|Map|Keys CurrentPercentChanges))
  (for _array_element _keys
    (Development|PrintString (Utilities|String|Append "Reducing: " (Utilities|String|EnumtoString (.StatToChange (Utilities|Struct|BreakStatChangesPercent (.Value (Utilities|Map|Find CurrentPercentChanges _array_element))))) " By: " (Utilities|String|ToString(Float) (* (- 1.0 (.PercentValue (Utilities|Struct|BreakStatChangesPercent (.Value (Utilities|Map|Find CurrentPercentChanges _array_element))))) 1e+02)) "%"))
    (Utilities|Map|Add (Variables|Default|GetPercentChangesStats) (Utilities|String|StringToName (Utilities|String|EnumtoString (.StatToChange (Utilities|Struct|BreakStatChangesPercent (.Value (Utilities|Map|Find CurrentPercentChanges _array_element)))))) (Math|Float|Clamp(Float) (* (.Value (Utilities|Map|Find (Variables|Default|GetPercentChangesStats) (Utilities|String|StringToName (Utilities|String|EnumtoString (.StatToChange (Utilities|Struct|BreakStatChangesPercent (.Value (Utilities|Map|Find CurrentPercentChanges _array_element)))))))) (.PercentValue (Utilities|Struct|BreakStatChangesPercent (.Value (Utilities|Map|Find CurrentPercentChanges _array_element))))) 0.0 9999.0))))

(event Custom|TickStats
  ;[1 0.9092 0.4678] Update Stats Logic
  (bind _output_get (Variables|Default|SetFlatChangesStats (Variables|Default|GetBaseStats)))
  (CallFunction|ApplyFlatStatChanges _output_get (Variables|Default|GetFlatStatChanges))
  (bind _output_get_2 (Variables|Default|SetPercentChangesStats (Variables|Default|GetFlatChangesStats)))
  (CallFunction|ApplyPercentStatChanges _output_get_2 (Variables|Default|GetPercentStatChanges))
  (bind _output_get_3 (Variables|Default|SetCurrentHealth (.Value (Utilities|Map|Find (Variables|Default|GetFinalStats) "CurrentHealth"))))
  (bind _output_get_4 (Variables|Default|SetFinalStats (Variables|Default|GetPercentChangesStats)))
  (Utilities|Map|Add _output_get_4 "CurrentHealth" _output_get_3)
  (CallFunction|UpdateStatsUI "NewEnumerator0" true 1e+01))

(event Custom|ApplyFlatStatChanges
  (params (StatsToChange :type Map%20of%20Names%20to%20Reals) (CurrentFlatChanges :type Map%20of%20Names%20to%20Structs))
  ;[1 0.9092 0.4678] Update Stats Logic
  (bind _keys (Utilities|Map|Keys CurrentFlatChanges))
  (for _array_element _keys
    (if (.IsBuff? (Utilities|Struct|BreakStatChangesFlat (.Value (Utilities|Map|Find CurrentFlatChanges _array_element))))
      (Utilities|Map|Add (Variables|Default|GetFlatChangesStats) (Utilities|String|StringToName (Utilities|String|EnumtoString (.StatToChange (Utilities|Struct|BreakStatChangesFlat (.Value (Utilities|Map|Find CurrentFlatChanges _array_element)))))) (Math|Float|Clamp(Float) (+ (.Value (Utilities|Map|Find StatsToChange (Utilities|String|StringToName (Utilities|String|EnumtoString (.StatToChange (Utilities|Struct|BreakStatChangesFlat (.Value (Utilities|Map|Find CurrentFlatChanges _array_element)))))))) (.FlatValue (Utilities|Struct|BreakStatChangesFlat (.Value (Utilities|Map|Find CurrentFlatChanges _array_element))))) 0.0 9999.0))
      (else
        (Utilities|Map|Add (Variables|Default|GetFlatChangesStats) (Utilities|String|StringToName (Utilities|String|EnumtoString (.StatToChange (Utilities|Struct|BreakStatChangesFlat (.Value (Utilities|Map|Find CurrentFlatChanges _array_element)))))) (Math|Float|Clamp(Float) (- (.Value (Utilities|Map|Find StatsToChange (Utilities|String|StringToName (Utilities|String|EnumtoString (.StatToChange (Utilities|Struct|BreakStatChangesFlat (.Value (Utilities|Map|Find CurrentFlatChanges _array_element)))))))) (.FlatValue (Utilities|Struct|BreakStatChangesFlat (.Value (Utilities|Map|Find CurrentFlatChanges _array_element))))) 0.0 9999.0))))))

(event Custom|DebuffApplied
  (params (Debuff%20Table :type Data%20Table%20Object%20Reference))
  ;[0.4589 0.1573 1] DebuffLogic
  (Utilities|FlowControl|Sequence
    (:then_0
      (Utilities|FlowControl|DoOnce false
        (:Completed
          (Utilities|Time|SetTimerbyEvent (delegate Custom|TickDebuffs) 1.0 true))))
    (:then_1
      (bind _outrownames (DataTable|GetDataTableRowNames Debuff%20Table))
      (for _array_element _outrownames
        (bind _returnvalue (Utilities|GetDataTableRow Debuff%20Table _array_element)
          (:then
            (Utilities|Map|Add (Variables|Default|GetDebuff) _array_element _returnvalue)))))))

(event EventBeginPlay)

(event EventApplyDamage
  (params (Physical%20Damage%20Amount :type Float%20%28double-precision%29) (Magical%20Damage%20Amount :type Float%20%28double-precision%29) (True%20Damage%20Amount :type Float%20%28double-precision%29) (Damage%20Type :type DamageTypeEnum%20Enum :default "NewEnumerator0") (Damage%20Causer :type Actor%20Object%20Reference) (Damage%20Victim :type Actor%20Object%20Reference) (Damage%20Method :type DamageMethodEnum%20Enum :default "NewEnumerator0") (Damage%20Method%20Percentage :type Float%20%28double-precision%29))
  ;[1 0.01151 0.1412] Damage Logic
  (switch Utilities|FlowControl|Switch|SwitchonDamageTypeEnum Damage%20Type
    (:NewEnumerator0
      (bind _damage_calculated_amount (CallFunction|CalculateDamageAmountUsingMethod Physical%20Damage%20Amount Damage%20Method Damage%20Method%20Percentage :!label _label))
      (bind _output_get (Variables|Default|SetPhysicalDamageAmount _damage_calculated_amount)))
    (:NewEnumerator1
      (bind _damage_calculated_amount_2 (CallFunction|CalculateDamageAmountUsingMethod Magical%20Damage%20Amount Damage%20Method Damage%20Method%20Percentage :!label _label_2))
      (bind _output_get_2 (Variables|Default|SetMagicalDamageAmount _damage_calculated_amount_2)))
    (:NewEnumerator2
      (Utilities|FlowControl|Sequence
        (:then_0
          (goto _label))
        (:then_1
          (goto _label_2))))
    (:NewEnumerator6
      (bind _damage_calculated_amount_3 (CallFunction|CalculateDamageAmountUsingMethod True%20Damage%20Amount Damage%20Method Damage%20Method%20Percentage :!label _label_3))
      (bind _output_get_3 (Variables|Default|SetTrueDamageAmount _damage_calculated_amount_3)))
    (:NewEnumerator7
      (Utilities|FlowControl|Sequence
        (:then_0
          (goto _label))
        (:then_1
          (goto _label_2))
        (:then_2
          (goto _label_3)))))
  (bind (_finalphysicaldamage _finalmagicaldamage _finaltruedamage) (CallFunction|CalculateDamageAmountUsingType _output_get _output_get_2 _output_get_3))
  (Variables|Default|SetFinal%20Physical%20Damage _finalphysicaldamage)
  (Variables|Default|SetFinal%20Magical%20Damage _finalmagicaldamage)
  (Variables|Default|SetFinal%20True%20Damage _finaltruedamage)
  (Utilities|FlowControl|Sequence
    (:then_0
      (if (not (<= (Variables|Default|GetFinal%20Physical%20Damage) 0.0))
        (Utilities|Map|Add (Variables|Default|GetFinalStats) "CurrentHealth" (Utilities|CalculatePhysicalDamageDone))
        (bind _returnvalue (Utilities|GetDataTableRow (Variables|Default|GetBaseStatsTable) "AttackDamage")
          (:then
            (CallFunction|DamageEffects "NewEnumerator0" (Variables|Default|GetFinal%20Physical%20Damage) "NewEnumerator0" (.TextColor (Utilities|Struct|BreakStats _returnvalue)))))))
    (:then_1
      (if (not (<= (Variables|Default|GetFinal%20Magical%20Damage) 0.0))
        (Utilities|Map|Add (Variables|Default|GetFinalStats) "CurrentHealth" (Utilities|CalculateMagicalDamageDone))
        (bind _returnvalue_2 (Utilities|GetDataTableRow (Variables|Default|GetBaseStatsTable) "AbilityPower")
          (:then
            (CallFunction|DamageEffects "NewEnumerator0" (Variables|Default|GetFinal%20Magical%20Damage) "NewEnumerator1" (.TextColor (Utilities|Struct|BreakStats _returnvalue_2)))))))
    (:then_2
      (if (not (<= (Variables|Default|GetFinal%20True%20Damage) 0.0))
        (Utilities|Map|Add (Variables|Default|GetFinalStats) "CurrentHealth" (Utilities|CalculateTrueDamageDone))
        (CallFunction|DamageEffects "NewEnumerator0" (Variables|Default|GetFinal%20True%20Damage) "NewEnumerator6" (Variables|Default|GetTrueDamageColor))))
    (:then_3
      (if (not (== (.Value (Utilities|Map|Find (Variables|Default|GetFinalStats) "CurrentHealth")) 0.0))
        (CallFunction|DamageEffects "NewEnumerator2" 0.0 "NewEnumerator6")
        (CallFunction|UpdateStatsUI "NewEnumerator7" false (.Value (Utilities|Map|Find (Variables|Default|GetFinalStats) "CurrentHealth")))
        (CallFunction|TickStats)))))

(event EventTick
  (params (DeltaSeconds :type Float%20%28single-precision%29)))

(fn CalculateDamageAmountUsingMethod
  (params (DamageAmount :type Float%20%28double-precision%29) (DamageMethod :type DamageMethodEnum%20Enum :default "NewEnumerator0") (DamagePercentage :type Float%20%28double-precision%29))
  (bind _finalstats (Variables|Default|GetFinalStats))
  (bind _value (Utilities|Map|Find _finalstats "MaxHealth"))
  (switch Utilities|FlowControl|Switch|SwitchonDamageMethodEnum DamageMethod
    (:NewEnumerator0
      (Variables|Default|SetDamageCalculated (* _value DamagePercentage)))
    (:NewEnumerator1
      (Variables|Default|SetDamageCalculated (* (.Value (Utilities|Map|Find _finalstats "CurrentHealth")) DamagePercentage)))
    (:NewEnumerator2
      (Variables|Default|SetDamageCalculated (* (- _value 0.0) DamagePercentage)))
    (:NewEnumerator6
      (Variables|Default|SetDamageCalculated DamageAmount)))
  (return (Variables|Default|GetDamageCalculated)))

(fn CalculateDamageAmountUsingType
  (params (PhysicalDamageAmount :type Float%20%28double-precision%29) (MagicalDamgeAmount :type Float%20%28double-precision%29) (TrueDamageAmount :type Float%20%28double-precision%29))
  (bind _finalstats (Variables|Default|GetFinalStats))
  (return (* PhysicalDamageAmount (/ 1e+02 (+ (.Value (Utilities|Map|Find _finalstats "Armour")) 1e+02))) (* MagicalDamgeAmount (/ 1e+02 (+ (.Value (Utilities|Map|Find _finalstats "MagicResist")) 1e+02))) TrueDamageAmount))