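; Health and stat component that loads base stats from a data table and handles damage and debuffs on its owner.
; ApplyDamage resolves amounts by flat or health-based method, mitigates them with base Armour or MagicResist, and messages the owner for effects.
; A one-second debuff timer counts down durations, dealing DOT or registering stat reductions.
; Another timer rebuilds FinalStats through flat and percent passes, also resetting CurrentHealth to MaxHealth each tick.
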(event Custom|InitStats
  (bind _basestats (Variables|Default|GetBaseStats))
  (bind _outrownames (DataTable|GetDataTableRowNames _basestats))
  (for _array_element _outrownames
    (bind _returnvalue (Utilities|GetDataTableRow _basestats _array_element)
      (:then
        (Utilities|Map|Add (Variables|Default|GetCurrentStats) _array_element (.Value (Utilities|Struct|BreakStats _returnvalue))))))
  (Variables|Default|SetCurrentHealth (.Value (Utilities|Map|Find (Variables|Default|GetCurrentStats) "MaxHealth")))
  (Utilities|Time|SetTimerbyFunctionName 0 "TickStats" 1.0 true))

(event Custom|DamageEffects
  (params (FXType :type DamageFXTypeEnum%20Enum :default "NewEnumerator0") (DamageNumbers :type Float%20%28double-precision%29) (DamageNumerType :type DamageTypeEnum%20Enum :default "NewEnumerator0") (Color :type Slate%20Color%20Structure))
  (Class|DamageSystem|DamageEffect(Message) (Components|GetOwner) FXType DamageNumbers DamageNumerType Color))

(event Custom|TickDebuffs
  (bind _debuff (Variables|Default|GetDebuff))
  (bind _debufflength (Variables|Default|GetDebuffLength))
  ;[0.4589 0.1573 1] DebuffLogic
  (bind _keys (Utilities|Map|Keys _debuff))
  (for _array_element _keys
    (if (Utilities|Map|Contains _debufflength _array_element)
      _
      (else
        (Utilities|Map|Add _debufflength _array_element (.LengthOfEntireDebuff (Utilities|Struct|BreakDebuff (.Value (Utilities|Map|Find _debuff _array_element)))))))
    (if (== (.Value (Utilities|Map|Find _debufflength _array_element)) 0.0)
      (Utilities|Map|Remove (Variables|Default|GetDebuff) _array_element)
      (Utilities|Map|Remove (Variables|Default|GetDebuffLength) _array_element)
      (switch Utilities|FlowControl|Switch|SwitchonDebuffEnum (.DebuffType (Utilities|Struct|BreakDebuff (.Value (Utilities|Map|Find _debuff _array_element))))
        (:NewEnumerator1
          (Utilities|Map|Remove (Variables|Default|GetFlatStatChanges) _array_element))
        (:NewEnumerator2
          (Utilities|Map|Remove (Variables|Default|GetPercentStatChanges) _array_element)))
      (else
        (bind _result (Math|Float|DecrementFloat (.Value (Utilities|Map|Find _debufflength _array_element)))
          (:%20%20
            (Utilities|Map|Add _debufflength _array_element _result)
            (switch Utilities|FlowControl|Switch|SwitchonDebuffEnum (.DebuffType (Utilities|Struct|BreakDebuff (.Value (Utilities|Map|Find _debuff _array_element))))
              (:NewEnumerator0
                (CallFunction|ApplyDamage (.DamageAmount (Utilities|Struct|BreakDebuff (.Value (Utilities|Map|Find _debuff _array_element)))) (.DamageAmount (Utilities|Struct|BreakDebuff (.Value (Utilities|Map|Find _debuff _array_element)))) (.DamageAmount (Utilities|Struct|BreakDebuff (.Value (Utilities|Map|Find _debuff _array_element)))) (.DamageType (Utilities|Struct|BreakDebuff (.Value (Utilities|Map|Find _debuff _array_element)))) 0 0 (.DamageMethod (Utilities|Struct|BreakDebuff (.Value (Utilities|Map|Find _debuff _array_element)))) (.DamagePercentage (Utilities|Struct|BreakDebuff (.Value (Utilities|Map|Find _debuff _array_element)))))
                (CallFunction|DamageEffects "NewEnumerator3" (.DamageAmount (Utilities|Struct|BreakDebuff (.Value (Utilities|Map|Find _debuff _array_element)))) (.DamageType (Utilities|Struct|BreakDebuff (.Value (Utilities|Map|Find _debuff _array_element))))))
              (:NewEnumerator1
                (Utilities|Map|Add (Variables|Default|GetFlatStatChanges) _array_element (Utilities|Struct|MakeStatChangesFlat (.FlatReductionAmount (Utilities|Struct|BreakDebuff (.Value (Utilities|Map|Find _debuff _array_element)))) (.StatToReduce (Utilities|Struct|BreakDebuff (.Value (Utilities|Map|Find _debuff _array_element)))) _array_element false)))
              (:NewEnumerator2
                (Utilities|Map|Add (Variables|Default|GetPercentStatChanges) _array_element (Utilities|Struct|MakeStatChangesPercent (.FlatReductionAmount (Utilities|Struct|BreakDebuff (.Value (Utilities|Map|Find _debuff _array_element)))) (.StatToReduce (Utilities|Struct|BreakDebuff (.Value (Utilities|Map|Find _debuff _array_element)))) _array_element false))))))))))

(event Custom|ApplyPercentStatChanges
  (params (StatsToChange :type Map%20of%20Names%20to%20Reals) (CurrentPercentChanges :type Map%20of%20Names%20to%20Structs))
  (bind _flatchangesstats (Variables|Default|GetFlatChangesStats))
  ;[0.4589 0.1573 1] DebuffLogic
  (bind _keys (Utilities|Map|Keys CurrentPercentChanges))
  (for _array_element _keys
    (Utilities|Map|Add _flatchangesstats (Utilities|Name|EnumtoName (.StatToChange (Utilities|Struct|BreakStatChangesPercent (.Value (Utilities|Map|Find CurrentPercentChanges _array_element))))) (Math|Float|Clamp(Float) (* (.Value (Utilities|Map|Find _flatchangesstats (Utilities|Name|EnumtoName (.StatToChange (Utilities|Struct|BreakStatChangesPercent (.Value (Utilities|Map|Find CurrentPercentChanges _array_element))))))) (.PercentValue (Utilities|Struct|BreakStatChangesPercent (.Value (Utilities|Map|Find CurrentPercentChanges _array_element))))) 0.0 9999.0))))

(event Custom|TickStats
  ;[0.4589 0.1573 1] DebuffLogic
  (bind _output_get (Variables|Default|SetFlatChangesStats (Variables|Default|GetCurrentStats)))
  (CallFunction|ApplyFlatStatChanges _output_get (Variables|Default|GetFlatStatChanges))
  (bind _output_get_2 (Variables|Default|SetPercentChangesStats (Variables|Default|GetFlatChangesStats)))
  (CallFunction|ApplyPercentStatChanges _output_get_2 (Variables|Default|GetPercentStatChanges))
  (bind _output_get_3 (Variables|Default|SetFinalStats (Variables|Default|GetPercentChangesStats)))
  (Variables|Default|SetCurrentHealth (.Value (Utilities|Map|Find _output_get_3 "MaxHealth"))))

(event Custom|ApplyFlatStatChanges
  (params (StatsToChange :type Map%20of%20Names%20to%20Reals) (CurrentFlatChanges :type Map%20of%20Names%20to%20Structs))
  (bind _flatchangesstats (Variables|Default|GetFlatChangesStats))
  ;[0.4589 0.1573 1] DebuffLogic
  (bind _keys (Utilities|Map|Keys CurrentFlatChanges))
  (for _array_element _keys
    (if (.IsBuff? (Utilities|Struct|BreakStatChangesFlat (.Value (Utilities|Map|Find CurrentFlatChanges _array_element))))
      (Utilities|Map|Add _flatchangesstats (Utilities|Name|EnumtoName (.StatToChange (Utilities|Struct|BreakStatChangesFlat (.Value (Utilities|Map|Find CurrentFlatChanges _array_element))))) (Math|Float|Clamp(Float) (+ (.Value (Utilities|Map|Find _flatchangesstats (Utilities|Name|EnumtoName (.StatToChange (Utilities|Struct|BreakStatChangesFlat (.Value (Utilities|Map|Find CurrentFlatChanges _array_element))))))) (.FlatValue (Utilities|Struct|BreakStatChangesFlat (.Value (Utilities|Map|Find CurrentFlatChanges _array_element))))) 0.0 9999.0))
      (else
        (Utilities|Map|Add _flatchangesstats (Utilities|Name|EnumtoName (.StatToChange (Utilities|Struct|BreakStatChangesFlat (.Value (Utilities|Map|Find CurrentFlatChanges _array_element))))) (Math|Float|Clamp(Float) (- (.Value (Utilities|Map|Find _flatchangesstats (Utilities|Name|EnumtoName (.StatToChange (Utilities|Struct|BreakStatChangesFlat (.Value (Utilities|Map|Find CurrentFlatChanges _array_element))))))) (.FlatValue (Utilities|Struct|BreakStatChangesFlat (.Value (Utilities|Map|Find CurrentFlatChanges _array_element))))) 0.0 9999.0))))))

(event Custom|DebuffApplied
  (params (NewParam :type Data%20Table%20Object%20Reference))
  ;[0.4589 0.1573 1] DebuffLogic
  (Utilities|FlowControl|Sequence
    (:then_0
      (Utilities|FlowControl|DoOnce false
        (:Completed
          (Utilities|Time|SetTimerbyEvent (delegate Custom|TickDebuffs) 1.0 true))))
    (:then_1
      (bind _outrownames (DataTable|GetDataTableRowNames NewParam))
      (for _array_element _outrownames
        (bind _returnvalue (Utilities|GetDataTableRow NewParam _array_element)
          (:then
            (Utilities|Map|Add (Variables|Default|GetDebuff) _array_element _returnvalue)))))))

(event EventBeginPlay)

(event EventTick
  (params (DeltaSeconds :type Float%20%28single-precision%29)))

(event EventApplyDamage
  (params (Physical%20Damage%20Amount :type Float%20%28double-precision%29) (Magical%20Damage%20Amount :type Float%20%28double-precision%29) (True%20Damage%20Amount :type Float%20%28double-precision%29) (Damage%20Type :type DamageTypeEnum%20Enum :default "NewEnumerator0") (Damage%20Causer :type Actor%20Object%20Reference) (Damage%20Victim :type Actor%20Object%20Reference) (Damage%20Method :type DamageMethodEnum%20Enum :default "NewEnumerator0") (Damage%20Method%20Percentage :type Float%20%28double-precision%29))
  ;[1 0.01151 0.1412] Damage Logic
  (switch Utilities|FlowControl|Switch|SwitchonDamageTypeEnum Damage%20Type
    (:NewEnumerator0
      (bind _damage_calculated_amount (CallFunction|CalculateDamageAmountUsingMethod Physical%20Damage%20Amount Damage%20Method Damage%20Method%20Percentage :!label _label))
      (bind _output_get (Variables|Default|SetPhysicalDamageAmount _damage_calculated_amount)))
    (:NewEnumerator1
      (bind _damage_calculated_amount_2 (CallFunction|CalculateDamageAmountUsingMethod Magical%20Damage%20Amount Damage%20Method Damage%20Method%20Percentage :!label _label_2))
      (bind _output_get_2 (Variables|Default|SetMagicalDamageAmount _damage_calculated_amount_2)))
    (:NewEnumerator2
      (Utilities|FlowControl|Sequence
        (:then_0
          (goto _label))
        (:then_1
          (goto _label_2))))
    (:NewEnumerator6
      (bind _damage_calculated_amount_3 (CallFunction|CalculateDamageAmountUsingMethod True%20Damage%20Amount Damage%20Method Damage%20Method%20Percentage :!label _label_3))
      (bind _output_get_3 (Variables|Default|SetTrueDamageAmount _damage_calculated_amount_3)))
    (:NewEnumerator7
      (Utilities|FlowControl|Sequence
        (:then_0
          (goto _label))
        (:then_1
          (goto _label_2))
        (:then_2
          (goto _label_3)))))
  (bind (_finalphysicaldamage _finalmagicaldamage _finaltruedamage) (CallFunction|CalculateDamageAmountUsingType _output_get _output_get_2 _output_get_3))
  (Utilities|FlowControl|Sequence
    (:then_0
      (Variables|Default|SetCurrentHealth (Math|Float|Clamp(Float) (- (Variables|Default|GetCurrentHealth) _finalphysicaldamage) 0.0 (.Value (Utilities|Map|Find (Variables|Default|GetFinalStats) "MaxHealth"))))
      (bind _returnvalue (Utilities|GetDataTableRow (Variables|Default|GetBaseStats) "AttackDamage")
        (:then
          (CallFunction|DamageEffects "NewEnumerator0" _finalphysicaldamage "NewEnumerator0" (.TextColor (Utilities|Struct|BreakStats _returnvalue))))))
    (:then_1
      (Variables|Default|SetCurrentHealth (Math|Float|Clamp(Float) (- (Variables|Default|GetCurrentHealth) _finalmagicaldamage) 0.0 (.Value (Utilities|Map|Find (Variables|Default|GetFinalStats) "MaxHealth"))))
      (bind _returnvalue_2 (Utilities|GetDataTableRow (Variables|Default|GetBaseStats) "AbilityPower")
        (:then
          (CallFunction|DamageEffects "NewEnumerator0" _finalmagicaldamage "NewEnumerator1" (.TextColor (Utilities|Struct|BreakStats _returnvalue_2))))))
    (:then_2
      (Variables|Default|SetCurrentHealth (Math|Float|Clamp(Float) (- (Variables|Default|GetCurrentHealth) _finaltruedamage) 0.0 (.Value (Utilities|Map|Find (Variables|Default|GetFinalStats) "MaxHealth"))))
      (CallFunction|DamageEffects "NewEnumerator0" _finaltruedamage "NewEnumerator6" (Variables|Default|GetTrueDamageColor)))
    (:then_3
      (if (not (== (Variables|Default|GetCurrentHealth) 0.0))
        (CallFunction|DamageEffects "NewEnumerator2" 0.0 "NewEnumerator6")))))

(event EventApplyDebuff
  (params (DebuffTable :type Data%20Table%20Object%20Reference) (Damage%20Causer :type Actor%20Object%20Reference) (Damage%20Victim :type Actor%20Object%20Reference))
  ;[0.4589 0.1573 1] DebuffLogic
  (Utilities|FlowControl|Sequence
    (:then_0
      (Utilities|FlowControl|DoOnce false
        (:Completed
          (Utilities|Time|SetTimerbyEvent (delegate Custom|TickDebuffs) 1.0 true))))
    (:then_1
      (bind _outrownames (DataTable|GetDataTableRowNames (stale Custom|DebuffApplied NewParam)))
      (for _array_element _outrownames
        (bind _returnvalue (Utilities|GetDataTableRow (stale Custom|DebuffApplied NewParam) _array_element)
          (:then
            (Utilities|Map|Add (Variables|Default|GetDebuff) _array_element _returnvalue)))))))

(fn CalculateDamageAmountUsingMethod
  (params (DamageAmount :type Float%20%28double-precision%29) (DamageMethod :type DamageMethodEnum%20Enum :default "NewEnumerator0") (DamagePercentage :type Float%20%28double-precision%29))
  (bind _currentstats (Variables|Default|GetCurrentStats))
  (bind _currenthealth (Variables|Default|GetCurrentHealth))
  (bind _value (Utilities|Map|Find _currentstats "MaxHealth"))
  (switch Utilities|FlowControl|Switch|SwitchonDamageMethodEnum DamageMethod
    (:NewEnumerator0
      (Variables|Default|SetDamageCalculated (* _value DamagePercentage)))
    (:NewEnumerator1
      (Variables|Default|SetDamageCalculated (* _currenthealth DamagePercentage)))
    (:NewEnumerator2
      (Variables|Default|SetDamageCalculated (* (- _value _currenthealth) DamagePercentage)))
    (:NewEnumerator6
      (Variables|Default|SetDamageCalculated DamageAmount)))
  (return (Variables|Default|GetDamageCalculated)))

(fn CalculateDamageAmountUsingType
  (params (PhysicalDamageAmount :type Float%20%28double-precision%29) (MagicalDamgeAmount :type Float%20%28double-precision%29) (TrueDamageAmount :type Float%20%28double-precision%29))
  (bind _currentstats (Variables|Default|GetCurrentStats))
  (return (* PhysicalDamageAmount (/ 1e+02 (+ (.Value (Utilities|Map|Find _currentstats "Armour")) 1e+02))) (* MagicalDamgeAmount (/ 1e+02 (+ (.Value (Utilities|Map|Find _currentstats "MagicResist")) 1e+02))) TrueDamageAmount))