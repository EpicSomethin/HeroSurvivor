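; BP_Parallax_Still is a background Blueprint that scrolls layered sprites on a plane to create a parallax effect.
; Each Tick it accumulates a time-based offset from ParallaxVelocity, independent of camera or player movement.
; It writes that offset into four material scalar parameters with decreasing multipliers, so each layer scrolls at its own speed for an illusion of depth.
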(event EventTick
  (params (DeltaSeconds :type Float%20%28single-precision%29))
  (bind _plane (Variables|Default|GetPlane))
  (Variables|Default|SetDelta%20Time DeltaSeconds)
  (Variables|Default|SetParallaxOffset (+ (Variables|Default|GetParallaxOffset) (* (Variables|Default|GetDelta%20Time) (Variables|Default|GetParallax%20Velocity))))
  (Rendering|Material|SetScalarParameterValueonMaterials _plane "Offset_0" (* (Variables|Default|GetParallaxOffset) 2.0))
  (Rendering|Material|SetScalarParameterValueonMaterials _plane "Offset_1" (* (Variables|Default|GetParallaxOffset) 1.2))
  (Rendering|Material|SetScalarParameterValueonMaterials _plane "Offset_2" (* (Variables|Default|GetParallaxOffset) 0.2))
  (Rendering|Material|SetScalarParameterValueonMaterials _plane "Offset_3" (* (Variables|Default|GetParallaxOffset) 0.1)))

(fn ConstructionScript)