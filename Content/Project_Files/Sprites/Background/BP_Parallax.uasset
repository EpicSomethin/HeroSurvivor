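; Parallax background actor for a side-scrolling view that follows a target supplied through LockTarget.
; Each tick it snaps to the target's X, keeping its own Y and Z, and accumulates an offset from the target's X velocity scaled by ParallaxVelocity.
; That offset drives four material scalar parameters on the Plane at decreasing rates, the last fixed at zero, giving layered depth from one mesh.
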(event Custom|LockTarget
  (params (Actor :type Actor%20Object%20Reference))
  (Utilities|IsValid Actor
    (:Is%20Valid
      (Variables|Default|SetObjective Actor))))

(event EventTick
  (params (DeltaSeconds :type Float%20%28single-precision%29))
  (bind _defaultsceneroot (Variables|Default|GetDefaultSceneRoot))
  (bind _objective (Variables|Default|GetObjective))
  (bind _plane (Variables|Default|GetPlane))
  (bind _returnvalue (Transformation|GetWorldLocation _defaultsceneroot))
  (Utilities|IsValid _objective
    (:Is%20Valid
      (if (== (.x (Transformation|GetVelocity _objective)) 0.0)
        _
        (else
          _))
      (Transformation|SetActorLocation (Math|Vector|MakeVector (.x (Transformation|GetActorLocation _objective)) (.y _returnvalue) (.z _returnvalue)) false false)
      (Variables|Default|SetDelta%20Time DeltaSeconds)
      (Variables|Default|SetParallaxOffset (+ (Variables|Default|GetParallaxOffset) (* (Variables|Default|GetDelta%20Time) (* (/ (.x (Transformation|GetVelocity _objective)) 2e+02) (Variables|Default|GetParallax%20Velocity)))))
      (if (> (Variables|Default|GetParallaxOffset) 1.0)
        _
        (else
          (Variables|Default|SetParallaxOffset (.Remainder (Math|Float|Division(WholeandRemainder) (Variables|Default|GetParallaxOffset) 1.0)))))
      (Rendering|Material|SetScalarParameterValueonMaterials _plane "Offset_0" (* (Variables|Default|GetParallaxOffset) 1.2))
      (Rendering|Material|SetScalarParameterValueonMaterials _plane "Offset_1" (* (Variables|Default|GetParallaxOffset) 0.6))
      (Rendering|Material|SetScalarParameterValueonMaterials _plane "Offset_2" (* (Variables|Default|GetParallaxOffset) 0.1))
      (Rendering|Material|SetScalarParameterValueonMaterials _plane "Offset_3" (* (Variables|Default|GetParallaxOffset) 0.0)))))

(fn ConstructionScript)